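; Flower actor that animates the emissive glow on its outer and inner petal meshes.
; BeginPlay creates and stores a dynamic material instance for the first material slot of each petal mesh.
; Tick calls Play on a timeline every frame, and the timeline's Emission track drives the Emission_L scalar parameter on both materials.
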(event `self.ReceiveBeginPlay`
  (bind _flower_testing_pettles_outter (`self.Flower_Testing_Pettles_Outter`))
  (bind _flower_testing_pettles_inner (`self.Flower_Testing_Pettles_Inner`))
  (bind _returnvalue (`PrimitiveComponent.CreateDynamicMaterialInstance` _flower_testing_pettles_outter 0 (`PrimitiveComponent.GetMaterial` _flower_testing_pettles_outter 0) "None"))
  (set `self.Mat` _returnvalue)
  (bind _returnvalue_2 (`PrimitiveComponent.CreateDynamicMaterialInstance` _flower_testing_pettles_inner 0 (`PrimitiveComponent.GetMaterial` _flower_testing_pettles_inner 0) "None"))
  (set `self.Mat_Two` _returnvalue_2))

(event `self.ReceiveTick`
  (params (DeltaSeconds :type "Float (single-precision)"))
  (bind (_direction _emission) (`Timeline|Timeline`)
    (:`Update`
      (`MaterialInstanceDynamic.SetScalarParameterValue` (`self.Mat`) "Emission_L" _emission)
      (`MaterialInstanceDynamic.SetScalarParameterValue` (`self.Mat_Two`) "Emission_L" _emission))))

(fn `UserConstructionScript`)